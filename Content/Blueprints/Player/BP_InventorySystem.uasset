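; Inventory actor that drives a 3D menu with Pause Menu, Inventory and Collectables levels stacked vertically.
; On Inventory, left/right input rotates the item carousel via timeline, one step of 360 degrees divided by the Scene's child count.
; Up/down input changes MenuState, and a timeline lerps MenuControllerPawn's height to that level's component.
; DoOnce and Gate nodes block repeat input until each animation finishes.
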(event `self.ReceiveBeginPlay`
  (`self.Update Total Items`))

(event `Update Total Items`
  (bind _output_get (set `self.Total Items` (`KismetArrayLibrary.Array_Length` (`SceneComponent.GetChildrenComponents` (`self.Scene`) false))))
  (set `self.Rotate Angle` (/ 360.0 (`KismetMathLibrary.Conv_IntToDouble` _output_get))))

(event `self.ReceiveTick`
  (params (DeltaSeconds :type "Float (single-precision)"))
  (set `self.Delta Seconds` DeltaSeconds))

(event `Rotate Left`
  (bind (_returnvalue_roll _returnvalue_pitch _returnvalue_yaw) (`KismetMathLibrary.BreakRotator` (`SceneComponent.K2_GetComponentRotation` (`self.Scene`))))
  (`self.Menu State Switch`
    (:`Inventory`
      (set `self.IsRotatingRight` false)
      (`/Engine/EditorBlueprintResources/StandardMacros.DoOnce` false :!label _label
        (:`Completed`
          (set `self.Current Rotation` _returnvalue_yaw)
          (bind (_direction _alpha) (`Timeline|Rotate` :!via `PlayFromStart`)
            (:`Update`
              (`SceneComponent.K2_SetWorldRotation` (`self.Scene`) (`KismetMathLibrary.MakeRotator` 0.0 0.0 (`KismetMathLibrary.Lerp` (`self.Current Rotation`) (+ (* (`self.Rotate Angle`) (`KismetMathLibrary.SelectFloat` -1.0 1.0 (`self.IsRotatingRight`))) (`self.Current Rotation`)) _alpha)) false false))
            (:`Finished`
              (`self.Reset Rotation`))))))))

(event `Rotate Right`
  (`self.Menu State Switch`
    (:`Inventory`
      (set `self.IsRotatingRight` true)
      (goto _label))))

(event `Reset Rotation`
  (goto _label :!via `Reset`))

(event `Move Up`
  (bind (_returnvalue_x _returnvalue_y _returnvalue_z) (`KismetMathLibrary.BreakVector` (`SceneComponent.K2_GetComponentLocation` (`self.MenuControllerPawn`))))
  (bind (_returnvalue_x_2 _returnvalue_y_2 _returnvalue_z_2) (`KismetMathLibrary.BreakVector` (`SceneComponent.K2_GetComponentLocation` (select `/Game/ThirdPersonBP/Blueprints/E_MenuState` (`self.Menu State`) :`NewEnumerator2` (`self.Pause Menu`) :`NewEnumerator0` (`self.Inventory`) :`NewEnumerator1` (`self.Collectables`)))))
  (`/Engine/EditorBlueprintResources/StandardMacros.Gate` false :!label _label_2
    (:`Exit`
      (`|ExecutionSequence`
        (:`then_0`
          (set `self.IsMovingUp` true)
          (`self.Menu State Switch`
            (:`Inventory`
              (set `self.Menu State` "NewEnumerator2")
              (bind (_direction _alpha) (`Timeline|Alpha` :!via `PlayFromStart` :!label _label_3)
                (:`Update`
                  (`SceneComponent.K2_SetWorldLocation` (`self.MenuControllerPawn`) (`KismetMathLibrary.MakeVector` 0.0 0.0 (`KismetMathLibrary.Lerp` _returnvalue_z _returnvalue_z_2 _alpha)) false false))
                (:`Finished`
                  (`self.Open Gates`))))
            (:`Collectables`
              (set `self.Menu State` "NewEnumerator0")
              (goto _label_3 :!via `PlayFromStart`))))
        (:`then_1`
          (`self.Close Gates` :!label _label_4))))))

(event `Open Gates`
  (`|ExecutionSequence`
    (:`then_0`
      (goto _label_2 :!via `Open`))
    (:`then_1`
      (goto _label_5 :!via `Open`))))

(event `Close Gates`
  (`|ExecutionSequence`
    (:`then_0`
      (goto _label_2 :!via `Close`))
    (:`then_1`
      (goto _label_5 :!via `Close`))))

(event `Move Down`
  (`/Engine/EditorBlueprintResources/StandardMacros.Gate` false :!label _label_5
    (:`Exit`
      (`|ExecutionSequence`
        (:`then_0`
          (set `self.IsMovingUp` false)
          (`self.Menu State Switch`
            (:`Pause Menu`
              (set `self.Menu State` "NewEnumerator0")
              (goto _label_3 :!via `PlayFromStart`))
            (:`Inventory`
              (set `self.Menu State` "NewEnumerator1")
              (goto _label_3 :!via `PlayFromStart`))))
        (:`then_1`
          (goto _label_4))))))

(fn `UserConstructionScript`)