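; Pawn possessed while the inventory menu is open, turning player input into inventory navigation and item use.
; BeginPlay caches the level's BP_InventorySystem and creates the WBP_Inventory widget, which AddWidget shows.
; Turn and move axes rotate or shift the inventory selection.
; Inventory and Action inputs hand possession back to BP_ThirdPersonCharacter and remove the HUD, resetting the camera or using the item respectively.
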(event `self.ReceiveBeginPlay`
  ;[1 1 1] Inventory
  (`|ExecutionSequence`
    (:`then_0`
      (bind _returnvalue (`GameplayStatics.GetActorOfClass` "/Game/Blueprints/Player/BP_InventorySystem.BP_InventorySystem_C"))
      (set `self.Inventory` _returnvalue))
    (:`then_1`
      (bind _returnvalue_2 (`|CreateWidget` "/Game/Blueprints/Widgets/WBP_Inventory.WBP_Inventory_C"))
      (set `self.InventoryHUD` _returnvalue_2))))

(event `InputAction|Inventory`
  (params (Key :type "Key Structure"))
  ;[1 1 1] Inventory
  (:`Pressed`
    (bind _returnvalue (`GameplayStatics.GetActorOfClass` "/Game/Blueprints/Player/BP_ThirdPersonCharacter.BP_ThirdPersonCharacter_C"))
    (`|ExecutionSequence`
      (:`then_0`
        (`Controller.Possess` (`GameplayStatics.GetPlayerController` 0) _returnvalue)
        (`self.Remove Widget`))
      (:`then_1`
        (`/Game/Blueprints/Player/BP_ThirdPersonCharacter.Set Camera` _returnvalue)))))

(event `InputAxis|TurnRight`
  (params (AxisValue :type "Float (single-precision)"))
  (bind _inventory (`self.Inventory`))
  ;[1 1 1] Left/Right Input
  (`/Engine/EditorBlueprintResources/StandardMacros.CompareFloat` AxisValue
    (:`>`
      (bind _asbp_inventory_system (cast `/Game/Blueprints/Player/BP_InventorySystem` _inventory))
      (`/Game/Blueprints/Player/BP_InventorySystem.Rotate Left` _asbp_inventory_system))
    (:`<`
      (bind _asbp_inventory_system_2 (cast `/Game/Blueprints/Player/BP_InventorySystem` _inventory))
      (`/Game/Blueprints/Player/BP_InventorySystem.Rotate Right` _asbp_inventory_system_2))))

(event `InputAxis|MoveForward`
  (params (AxisValue :type "Float (single-precision)"))
  (bind _inventory (`self.Inventory`))
  ;[1 1 1] Up/Down Input
  (`/Engine/EditorBlueprintResources/StandardMacros.CompareFloat` AxisValue
    (:`>`
      (bind _asbp_inventory_system (cast `/Game/Blueprints/Player/BP_InventorySystem` _inventory))
      (`/Game/Blueprints/Player/BP_InventorySystem.Move Up` _asbp_inventory_system))
    (:`<`
      (bind _asbp_inventory_system_2 (cast `/Game/Blueprints/Player/BP_InventorySystem` _inventory))
      (`/Game/Blueprints/Player/BP_InventorySystem.Move Down` _asbp_inventory_system_2))))

(event `Add Widget`
  (`/Engine/EditorBlueprintResources/StandardMacros.IsValid` (`self.InventoryHUD`)
    (:`Is Valid`
      _)
    (:`Is Not Valid`
      (bind _returnvalue (`|CreateWidget` "/Game/Blueprints/Widgets/WBP_Inventory.WBP_Inventory_C" (`GameplayStatics.GetPlayerController` 0)))
      (bind _output_get (set `self.InventoryHUD` _returnvalue))))
  (`UserWidget.AddToViewport` _output_get 0))

(event `Remove Widget`
  (`Widget.RemoveFromParent` (`self.InventoryHUD`)))

(event `InputAction|Action`
  (params (Key :type "Key Structure"))
  (:`Pressed`
    (bind _returnvalue (`GameplayStatics.GetActorOfClass` "/Game/Blueprints/Player/BP_ThirdPersonCharacter.BP_ThirdPersonCharacter_C"))
    (`/Game/Blueprints/Player/BP_ThirdPersonCharacter.Use Item` _returnvalue (`self.Inventory`))
    (`Controller.Possess` (`GameplayStatics.GetPlayerController` 0) _returnvalue)
    (`self.Remove Widget`)))

(fn `UserConstructionScript`)