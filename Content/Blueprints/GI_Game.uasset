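; GI_Game is a Game Instance that persists the player's settings through a BP_SettingsSave save object.
; On Init it loads the settings slot, or creates and immediately saves a fresh save object when none loads as that class.
; On Shutdown it writes the held SettingsSave back to the slot, printing debug messages on load success or save failure.
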(event `self.ReceiveInit`
  (`self.Load Settings`))

(event `self.ReceiveShutdown`
  (`self.Save Settings`))

(fn `Load Settings`
  (bind _returnvalue (`GameplayStatics.LoadGameFromSlot` (`self.Settings Slot`)))
  (bind _asbp_settings_save (cast `/Game/Blueprints/BP_SettingsSave` _returnvalue)
    (:`then`
      (set `self.Settings Save` _asbp_settings_save)
      (`KismetSystemLibrary.PrintString` "Load Settings Success"))
    (:`CastFailed`
      (bind _returnvalue_2 (`GameplayStatics.CreateSaveGameObject` "/Game/Blueprints/BP_SettingsSave.BP_SettingsSave_C"))
      (bind _output_get (set `self.Settings Save` _returnvalue_2))
      (bind _returnvalue_3 (`GameplayStatics.SaveGameToSlot` _output_get (`self.Settings Slot`)))
      (if (not _returnvalue_3)
        (`KismetSystemLibrary.PrintString` "Failed to Load Settings. Check GI_Game")))))

(fn `Save Settings`
  (bind _returnvalue (`GameplayStatics.SaveGameToSlot` (`self.Settings Save`) (`self.Settings Slot`)))
  (if (not _returnvalue)
    (`KismetSystemLibrary.PrintString` "Failed to Save Settings. Check GI_Game")))