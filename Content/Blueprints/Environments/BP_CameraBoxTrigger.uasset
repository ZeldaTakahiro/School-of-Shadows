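; BP_CameraBoxTrigger is a level trigger volume that switches the player's view to an assigned camera when the player pawn enters its box.
; On overlap it sets the camera as the player controller's view target and records itself as the third-person character's LastCameraTriggered.
; A DoOnce gate prevents repeat switches until the player leaves the box, which resets it.
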(event `self.Box.OnComponentBeginOverlap`
  (params (OverlappedComponent :type "PrimitiveComponent Object Reference") (OtherActor :type "Actor Object Reference") (OtherComp :type "PrimitiveComponent Object Reference") (OtherBodyIndex :type Integer) (bFromSweep :type Boolean) (SweepResult :type "HitResult Structure (by ref)"))
  ;[1 1 1] Setting Overlapping Trigger
  (if (== OtherActor (`GameplayStatics.GetPlayerPawn` 0))
    (`/Engine/EditorBlueprintResources/StandardMacros.DoOnce` false :!label _label
      (:`Completed`
        (`PlayerController.SetViewTargetWithBlend` (`GameplayStatics.GetPlayerController` 0) (`self.Camera`) 0.0 "VTBlend_Linear" 0.0 false)
        (bind _asbp_third_person_character (cast `/Game/Blueprints/Player/BP_ThirdPersonCharacter` (`GameplayStatics.GetPlayerPawn` 0)))
        (set `/Game/Blueprints/Player/BP_ThirdPersonCharacter.LastCameraTriggered` self _asbp_third_person_character)))))

(event `self.Box.OnComponentEndOverlap`
  (params (OverlappedComponent :type "PrimitiveComponent Object Reference") (OtherActor :type "Actor Object Reference") (OtherComp :type "PrimitiveComponent Object Reference") (OtherBodyIndex :type Integer))
  ;[1 1 1] Setting Overlapping Trigger
  (if (== OtherActor (`GameplayStatics.GetPlayerPawn` 0))
    (goto _label :!via `Reset`)))

(fn `UserConstructionScript`)