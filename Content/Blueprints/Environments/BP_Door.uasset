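; BP_Door is a door actor that teleports the player to its opposite side behind a screen fade.
; Left and right interaction volumes record the player's side, register the door as the character's OverlappingTrigger and update its header.
; Teleport plays the HUD fade while a short delay precedes moving the pawn to the other side's point and arrow rotation.
; A DoOnce blocks retriggering until the fade ends.
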(event `self.L_Interaction.OnComponentBeginOverlap`
  (params (OverlappedComponent :type "PrimitiveComponent Object Reference") (OtherActor :type "Actor Object Reference") (OtherComp :type "PrimitiveComponent Object Reference") (OtherBodyIndex :type Integer) (bFromSweep :type Boolean) (SweepResult :type "HitResult Structure (by ref)"))
  (if (== OtherActor (`GameplayStatics.GetPlayerPawn` 0))
    (set `self.IsInteractable` true)
    (set `self.IsOverlappingRight` false)
    (bind _asthird_person_character (cast `/Game/Blueprints/Player/ThirdPersonCharacter` (`GameplayStatics.GetPlayerPawn` 0)))
    (set `/Game/Blueprints/Player/ThirdPersonCharacter.OverlappingTrigger` self _asthird_person_character)
    (`/Game/Blueprints/Player/ThirdPersonCharacter.UpdateHeader` _asthird_person_character (`self.Billboard`))))

(event `self.L_Interaction.OnComponentEndOverlap`
  (params (OverlappedComponent :type "PrimitiveComponent Object Reference") (OtherActor :type "Actor Object Reference") (OtherComp :type "PrimitiveComponent Object Reference") (OtherBodyIndex :type Integer))
  (if (== OtherActor (`GameplayStatics.GetPlayerPawn` 0))
    (set `self.IsInteractable` false)
    (bind _asthird_person_character (cast `/Game/Blueprints/Player/ThirdPersonCharacter` (`GameplayStatics.GetPlayerPawn` 0)))
    (set `/Game/Blueprints/Player/ThirdPersonCharacter.OverlappingTrigger` null _asthird_person_character)
    (`/Game/Blueprints/Player/ThirdPersonCharacter.UpdateHeader` _asthird_person_character null)))

(event `self.R_Interaction.OnComponentBeginOverlap`
  (params (OverlappedComponent :type "PrimitiveComponent Object Reference") (OtherActor :type "Actor Object Reference") (OtherComp :type "PrimitiveComponent Object Reference") (OtherBodyIndex :type Integer) (bFromSweep :type Boolean) (SweepResult :type "HitResult Structure (by ref)"))
  (if (== OtherActor (`GameplayStatics.GetPlayerPawn` 0))
    (set `self.IsInteractable` true)
    (set `self.IsOverlappingRight` true)
    (bind _asthird_person_character (cast `/Game/Blueprints/Player/ThirdPersonCharacter` (`GameplayStatics.GetPlayerPawn` 0)))
    (set `/Game/Blueprints/Player/ThirdPersonCharacter.OverlappingTrigger` self _asthird_person_character)
    (`/Game/Blueprints/Player/ThirdPersonCharacter.UpdateHeader` _asthird_person_character (`self.Billboard`))))

(event `self.R_Interaction.OnComponentEndOverlap`
  (params (OverlappedComponent :type "PrimitiveComponent Object Reference") (OtherActor :type "Actor Object Reference") (OtherComp :type "PrimitiveComponent Object Reference") (OtherBodyIndex :type Integer))
  (if (== OtherActor (`GameplayStatics.GetPlayerPawn` 0))
    (set `self.IsInteractable` false)
    (bind _asthird_person_character (cast `/Game/Blueprints/Player/ThirdPersonCharacter` (`GameplayStatics.GetPlayerPawn` 0)))
    (set `/Game/Blueprints/Player/ThirdPersonCharacter.OverlappingTrigger` null _asthird_person_character)
    (`/Game/Blueprints/Player/ThirdPersonCharacter.UpdateHeader` _asthird_person_character null)))

(event `Teleport`
  (bind _returnvalue (`GameplayStatics.GetPlayerPawn` 0))
  (`/Engine/EditorBlueprintResources/StandardMacros.DoOnce` false :!label _label
    (:`Completed`
      (`|ExecutionSequence`
        (:`then_0`
          (`KismetSystemLibrary.Delay` 0.375)
          (if (`self.IsOverlappingRight`)
            (`self.K2_SetActorLocationAndRotation` _returnvalue (`SceneComponent.K2_GetComponentLocation` (`self.L_Teleport`)) (`SceneComponent.K2_GetComponentRotation` (`self.L_Arrow`)) false true)
            (else
              (`self.K2_SetActorLocationAndRotation` _returnvalue (`SceneComponent.K2_GetComponentLocation` (`self.R_Teleport`)) (`SceneComponent.K2_GetComponentRotation` (`self.R_Arrow`)) false true))))
        (:`then_1`
          (bind _foundwidgets (`WidgetBlueprintLibrary.GetAllWidgetsOfClass` "/Game/Blueprints/Widgets/InGame/WBP_HUD.WBP_HUD_C" false))
          (bind _wbp_screenfade (`/Game/Blueprints/Widgets/InGame/WBP_HUD.WBP_ScreenFade` (`|GetArrayItem` _foundwidgets)))
          (bind _fadeinout (`/Game/Blueprints/Widgets/WBP_ScreenFade.FadeInOut` _wbp_screenfade))
          (`UserWidget.PlayAnimation` _wbp_screenfade _fadeinout 0.0 1 "Forward" 1.0 false)
          (`KismetSystemLibrary.Delay` (+ (`WidgetAnimation.GetEndTime` _fadeinout) 0.25))
          (`self.Reset Teleport`))))))

(event `Reset Teleport`
  (goto _label :!via `Reset`))

(fn `UserConstructionScript`)