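; BP_ItemBoxTrigger is an interactable trigger volume that can show dialogue and check for a required item.
; When the player pawn enters or leaves the box, it toggles interactability, sets or clears the character's OverlappingTrigger and updates its header, using the Billboard on entry.
; BeginDialogue passes its dialogue to the first WBP_DialogueBox found and starts it.
; CheckItem compares an item ID to RequiredItemID and only prints the result.
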(event `self.Box.OnComponentBeginOverlap`
  (params (OverlappedComponent :type "PrimitiveComponent Object Reference") (OtherActor :type "Actor Object Reference") (OtherComp :type "PrimitiveComponent Object Reference") (OtherBodyIndex :type Integer) (bFromSweep :type Boolean) (SweepResult :type "HitResult Structure (by ref)"))
  ;[1 1 1] Setting Overlapping Trigger
  (if (== OtherActor (`GameplayStatics.GetPlayerPawn` 0))
    (set `self.IsInteractable` true)
    (bind _asbp_third_person_character (cast `/Game/Blueprints/Player/BP_ThirdPersonCharacter` (`GameplayStatics.GetPlayerPawn` 0)))
    (set `/Game/Blueprints/Player/BP_ThirdPersonCharacter.OverlappingTrigger` self _asbp_third_person_character)
    (`/Game/Blueprints/Player/BP_ThirdPersonCharacter.UpdateHeader` _asbp_third_person_character (`self.Billboard`))))

(event `self.Box.OnComponentEndOverlap`
  (params (OverlappedComponent :type "PrimitiveComponent Object Reference") (OtherActor :type "Actor Object Reference") (OtherComp :type "PrimitiveComponent Object Reference") (OtherBodyIndex :type Integer))
  ;[1 1 1] Setting Overlapping Trigger
  (if (== OtherActor (`GameplayStatics.GetPlayerPawn` 0))
    (set `self.IsInteractable` false)
    (bind _asbp_third_person_character (cast `/Game/Blueprints/Player/BP_ThirdPersonCharacter` (`GameplayStatics.GetPlayerPawn` 0)))
    (set `/Game/Blueprints/Player/BP_ThirdPersonCharacter.OverlappingTrigger` null _asbp_third_person_character)
    (`/Game/Blueprints/Player/BP_ThirdPersonCharacter.UpdateHeader` _asbp_third_person_character null)))

(event `Begin Dialogue`
  ;[1 1 1] Begin Dialogue
  (bind _foundwidgets (`WidgetBlueprintLibrary.GetAllWidgetsOfClass` "/Game/Blueprints/Widgets/InGame/WBP_DialogueBox.WBP_DialogueBox_C" false))
  (bind _output (`|GetArrayItem` _foundwidgets))
  (set `/Game/Blueprints/Widgets/InGame/WBP_DialogueBox.DialogueList` (`self.Dialogue`) _output)
  (`/Game/Blueprints/Widgets/InGame/WBP_DialogueBox.Begin Dialogue` _output))

(event `Check Item`
  (params (`Item ID` :type Integer))
  (if (== `Item ID` (`self.Required Item ID`))
    (`KismetSystemLibrary.PrintString` "Success")
    (else
      (`KismetSystemLibrary.PrintString` "No Success"))))

(fn `UserConstructionScript`)